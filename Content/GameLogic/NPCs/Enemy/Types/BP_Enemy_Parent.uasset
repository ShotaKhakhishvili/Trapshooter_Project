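; BP_Enemy_Parent is an enemy NPC base Blueprint that handles health and an overhead health bar.
; On BeginPlay it fills HP, caches the player character and links itself to the WGT_EnemyHealth widget.
; ChangeHealth applies a delta while the player is alive, updates the bar text and destroys the enemy at exactly zero HP.
; Tick rotates the widget component in pitch and yaw to face the player's camera.
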(event EventChangeHealth
  (params (Delta :type Integer))
  (if (not (Variables|/Game/TopDown/Blueprints/BP_TopDownCharacter.BP_TopDownCharacter_C|GetDead (Variables|Default|GetPlayer)))
    (bind _output_get (Variables|Default|SetHP_Current (+ Delta (Variables|Default|GetHP_Current))))
    (Utilities|RefreshHealthBar)
    (if (== _output_get 0)
      (Actor|DestroyActor))))

(event EventBeginPlay
  (Variables|Default|SetHP_Current (Variables|Default|GetHP_Max))
  (bind _asbp_top_down_character (Utilities|Casting|CastToBP_TopDownCharacter (Game|GetPlayerCharacter 0)))
  (Variables|Default|SetPlayer _asbp_top_down_character)
  (Utilities|SetupHPBar)
  (Utilities|RefreshHealthBar))

(event EventTick
  (params (DeltaSeconds :type Float%20%28single-precision%29))
  (Utilities|SetWidgetRotation))

(fn ConstructionScript)